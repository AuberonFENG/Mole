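; Player character for a multiplayer whack-a-mole game, letting a player control the moles in nine holes.
; Nine Enhanced Input key actions each map to a hole, raising its mole on press and lowering it on release or cancel, if that mole is valid.
; Two custom events add incoming points to separate running totals, Score and MoleScore.
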(event `CE_MoleGetScore`
  (params (NewParam :type "Float (double-precision)"))
  (set `self.moleScore` (+ NewParam (`self.moleScore`))))

(event `CE_GetScore`
  (params (NewParam :type "Float (double-precision)"))
  (set `self.score` (+ NewParam (`self.score`))))

(event `EnhancedInput|/Game/Multiplayer/Key/IA_Key1`
  (params (ActionValue :type Boolean) (ElapsedSeconds :type "Float (double-precision)") (TriggeredSeconds :type "Float (double-precision)") (InputAction :type "InputAction Object Reference" :default "/Game/Multiplayer/Key/IA_Key1.IA_Key1"))
  (bind _mole (`/Game/Multiplayer/Blueprint/BP_Hole.mole` (`self.hole_1`)))
  (:`Started`
    (`/Engine/EditorBlueprintResources/StandardMacros.IsValid` _mole
      (:`Is Valid`
        (`/Game/Multiplayer/Blueprint/BP_Mole.CE_Up` _mole))))
  (:`Canceled`
    (`/Engine/EditorBlueprintResources/StandardMacros.IsValid` _mole :!label _label
      (:`Is Valid`
        (`/Game/Multiplayer/Blueprint/BP_Mole.CE_Down` _mole))))
  (:`Completed`
    (goto _label)))

(event `EnhancedInput|/Game/Multiplayer/Key/IA_Key2`
  (params (ActionValue :type Boolean) (ElapsedSeconds :type "Float (double-precision)") (TriggeredSeconds :type "Float (double-precision)") (InputAction :type "InputAction Object Reference" :default "/Game/Multiplayer/Key/IA_Key2.IA_Key2"))
  (bind _mole (`/Game/Multiplayer/Blueprint/BP_Hole.mole` (`self.hole_2`)))
  (:`Started`
    (`/Engine/EditorBlueprintResources/StandardMacros.IsValid` _mole
      (:`Is Valid`
        (`/Game/Multiplayer/Blueprint/BP_Mole.CE_Up` _mole))))
  (:`Canceled`
    (`/Engine/EditorBlueprintResources/StandardMacros.IsValid` _mole :!label _label_2
      (:`Is Valid`
        (`/Game/Multiplayer/Blueprint/BP_Mole.CE_Down` _mole))))
  (:`Completed`
    (goto _label_2)))

(event `EnhancedInput|/Game/Multiplayer/Key/IA_Key3`
  (params (ActionValue :type Boolean) (ElapsedSeconds :type "Float (double-precision)") (TriggeredSeconds :type "Float (double-precision)") (InputAction :type "InputAction Object Reference" :default "/Game/Multiplayer/Key/IA_Key3.IA_Key3"))
  (bind _mole (`/Game/Multiplayer/Blueprint/BP_Hole.mole` (`self.hole_3`)))
  (:`Started`
    (`/Engine/EditorBlueprintResources/StandardMacros.IsValid` _mole
      (:`Is Valid`
        (`/Game/Multiplayer/Blueprint/BP_Mole.CE_Up` _mole))))
  (:`Canceled`
    (`/Engine/EditorBlueprintResources/StandardMacros.IsValid` _mole :!label _label_3
      (:`Is Valid`
        (`/Game/Multiplayer/Blueprint/BP_Mole.CE_Down` _mole))))
  (:`Completed`
    (goto _label_3)))

(event `EnhancedInput|/Game/Multiplayer/Key/IA_Key4`
  (params (ActionValue :type Boolean) (ElapsedSeconds :type "Float (double-precision)") (TriggeredSeconds :type "Float (double-precision)") (InputAction :type "InputAction Object Reference" :default "/Game/Multiplayer/Key/IA_Key4.IA_Key4"))
  (bind _mole (`/Game/Multiplayer/Blueprint/BP_Hole.mole` (`self.hole_4`)))
  (:`Started`
    (`/Engine/EditorBlueprintResources/StandardMacros.IsValid` _mole
      (:`Is Valid`
        (`/Game/Multiplayer/Blueprint/BP_Mole.CE_Up` _mole))))
  (:`Canceled`
    (`/Engine/EditorBlueprintResources/StandardMacros.IsValid` _mole :!label _label_4
      (:`Is Valid`
        (`/Game/Multiplayer/Blueprint/BP_Mole.CE_Down` _mole))))
  (:`Completed`
    (goto _label_4)))

(event `EnhancedInput|/Game/Multiplayer/Key/IA_Key5`
  (params (ActionValue :type Boolean) (ElapsedSeconds :type "Float (double-precision)") (TriggeredSeconds :type "Float (double-precision)") (InputAction :type "InputAction Object Reference" :default "/Game/Multiplayer/Key/IA_Key5.IA_Key5"))
  (bind _mole (`/Game/Multiplayer/Blueprint/BP_Hole.mole` (`self.hole_5`)))
  (:`Started`
    (`/Engine/EditorBlueprintResources/StandardMacros.IsValid` _mole
      (:`Is Valid`
        (`/Game/Multiplayer/Blueprint/BP_Mole.CE_Up` _mole))))
  (:`Canceled`
    (`/Engine/EditorBlueprintResources/StandardMacros.IsValid` _mole :!label _label_5
      (:`Is Valid`
        (`/Game/Multiplayer/Blueprint/BP_Mole.CE_Down` _mole))))
  (:`Completed`
    (goto _label_5)))

(event `EnhancedInput|/Game/Multiplayer/Key/IA_Key6`
  (params (ActionValue :type Boolean) (ElapsedSeconds :type "Float (double-precision)") (TriggeredSeconds :type "Float (double-precision)") (InputAction :type "InputAction Object Reference" :default "/Game/Multiplayer/Key/IA_Key6.IA_Key6"))
  (bind _mole (`/Game/Multiplayer/Blueprint/BP_Hole.mole` (`self.hole_6`)))
  (:`Started`
    (`/Engine/EditorBlueprintResources/StandardMacros.IsValid` _mole
      (:`Is Valid`
        (`/Game/Multiplayer/Blueprint/BP_Mole.CE_Up` _mole))))
  (:`Canceled`
    (`/Engine/EditorBlueprintResources/StandardMacros.IsValid` _mole :!label _label_6
      (:`Is Valid`
        (`/Game/Multiplayer/Blueprint/BP_Mole.CE_Down` _mole))))
  (:`Completed`
    (goto _label_6)))

(event `EnhancedInput|/Game/Multiplayer/Key/IA_Key7`
  (params (ActionValue :type Boolean) (ElapsedSeconds :type "Float (double-precision)") (TriggeredSeconds :type "Float (double-precision)") (InputAction :type "InputAction Object Reference" :default "/Game/Multiplayer/Key/IA_Key7.IA_Key7"))
  (bind _mole (`/Game/Multiplayer/Blueprint/BP_Hole.mole` (`self.hole_7`)))
  (:`Started`
    (`/Engine/EditorBlueprintResources/StandardMacros.IsValid` _mole
      (:`Is Valid`
        (`/Game/Multiplayer/Blueprint/BP_Mole.CE_Up` _mole))))
  (:`Canceled`
    (`/Engine/EditorBlueprintResources/StandardMacros.IsValid` _mole :!label _label_7
      (:`Is Valid`
        (`/Game/Multiplayer/Blueprint/BP_Mole.CE_Down` _mole))))
  (:`Completed`
    (goto _label_7)))

(event `EnhancedInput|/Game/Multiplayer/Key/IA_Key8`
  (params (ActionValue :type Boolean) (ElapsedSeconds :type "Float (double-precision)") (TriggeredSeconds :type "Float (double-precision)") (InputAction :type "InputAction Object Reference" :default "/Game/Multiplayer/Key/IA_Key8.IA_Key8"))
  (bind _mole (`/Game/Multiplayer/Blueprint/BP_Hole.mole` (`self.hole_8`)))
  (:`Started`
    (`/Engine/EditorBlueprintResources/StandardMacros.IsValid` _mole
      (:`Is Valid`
        (`/Game/Multiplayer/Blueprint/BP_Mole.CE_Up` _mole))))
  (:`Canceled`
    (`/Engine/EditorBlueprintResources/StandardMacros.IsValid` _mole :!label _label_8
      (:`Is Valid`
        (`/Game/Multiplayer/Blueprint/BP_Mole.CE_Down` _mole))))
  (:`Completed`
    (goto _label_8)))

(event `EnhancedInput|/Game/Multiplayer/Key/IA_Key9`
  (params (ActionValue :type Boolean) (ElapsedSeconds :type "Float (double-precision)") (TriggeredSeconds :type "Float (double-precision)") (InputAction :type "InputAction Object Reference" :default "/Game/Multiplayer/Key/IA_Key9.IA_Key9"))
  (bind _mole (`/Game/Multiplayer/Blueprint/BP_Hole.mole` (`self.hole_9`)))
  (:`Started`
    (`/Engine/EditorBlueprintResources/StandardMacros.IsValid` _mole
      (:`Is Valid`
        (`/Game/Multiplayer/Blueprint/BP_Mole.CE_Up` _mole))))
  (:`Canceled`
    (`/Engine/EditorBlueprintResources/StandardMacros.IsValid` _mole :!label _label_9
      (:`Is Valid`
        (`/Game/Multiplayer/Blueprint/BP_Mole.CE_Down` _mole))))
  (:`Completed`
    (goto _label_9)))

(fn `UserConstructionScript`)