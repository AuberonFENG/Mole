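; Whack-a-mole actor that rises and sinks on timelines, passing scores to BP_MultiplayerCharacter.
; An enum state gates movement, and sinking resumes from the saved rise position.
; While fully up, Tick awards mole score every 0.2 seconds.
; Clicking a non-hidden mole starts a combo; later hits show a combo widget, award player score, play effects and lower it, while clicking a hidden mole resets the combo.
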(event `OnClicked_Event` :!signature `self.OnClicked`
  (params (TouchedActor :type "Actor Object Reference") (ButtonPressed :type "Key Structure" :default "None")))

(event `self.ReceiveBeginPlay`
  ;[1 1 1] 游戏开始时切换控制
  (set `self.bpMultiplayer` (cast `/Game/Characters/BP_MultiplayerCharacter` (`GameplayStatics.GetPlayerCharacter` 0) :!pure true))
  (set `self.ComboCounter` 0)
  (set `self.IsComboActive` false))

(event `self.ReceiveTick`
  (params (DeltaSeconds :type "Float (single-precision)"))
  ;[1 1 1] 每帧调用地鼠得分
  (if (`self.tickLocked`)
    _
    (elif (`|EnumEquality` (`self.animState`) "NewEnumerator3")
      (`/Game/Characters/BP_MultiplayerCharacter.CE_MoleGetScore` (`self.bpMultiplayer`) (`self.moleScore`))
      (set `self.tickLocked` true)
      (`KismetSystemLibrary.Delay` 0.2)
      (set `self.tickLocked` false))))

(event `CE_Up`
  (bind (_beginlocation_x _beginlocation_y _beginlocation_z) (`KismetMathLibrary.BreakVector` (`self.beginLocation`)))
  (if (`|EnumEquality` (`self.animState`) "NewEnumerator2")
    (`TimelineComponent.SetPlayRate` (`self.Timeline_Up`) (`self.playRate`))
    (set `self.animState` "NewEnumerator0")
    (set `self.beginLocation` (`self.K2_GetActorLocation`))
    (bind (_direction _up) (`Timeline|Timeline_Up` :!via `PlayFromStart` :!label _label)
      (:`Update`
        (set `self.upTime` _up)
        (`self.K2_SetActorLocation` (`KismetMathLibrary.MakeVector` _beginlocation_x _beginlocation_y (+ _beginlocation_z (* _up (`self.height`)))))
        (`GameplayStatics.PlaySound2D` "/Game/SoundEffects/mixkit-martial-arts-fast-punch-2047.mixkit-martial-arts-fast-punch-2047" 1.0 1.0 0.0 null null))
      (:`Finished`
        (`self.CE_Stay`)))))

(event `CE_StopUp`
  (goto _label :!via `Stop`))

(event `CE_Stay`
  (set `self.animState` "NewEnumerator3"))

(event `CE_Down`
  (bind _timeline_down (`self.Timeline_Down`))
  (bind (_beginlocation_x _beginlocation_y _beginlocation_z) (`KismetMathLibrary.BreakVector` (`self.beginLocation`)))
  (if (`|EnumInequality` (`self.animState`) "NewEnumerator2")
    (if (`|EnumInequality` (`self.animState`) "NewEnumerator1")
      (set `self.animState` "NewEnumerator1")
      (`self.CE_StopUp`)
      (`TimelineComponent.SetPlayRate` _timeline_down (* (`self.playRate`) -1.0))
      (`TimelineComponent.SetPlaybackPosition` _timeline_down (`self.upTime`) true true)
      (bind (_direction _down) (`Timeline|Timeline_Down`)
        (:`Update`
          (`self.K2_SetActorLocation` (`KismetMathLibrary.MakeVector` _beginlocation_x _beginlocation_y (+ _beginlocation_z (* _down (`self.height`))))))
        (:`Finished`
          (set `self.animState` "NewEnumerator2"))))))

(event `self.ReceiveActorOnClicked`
  (params (ButtonPressed :type "Key Structure"))
  (bind (_beginlocation_x _beginlocation_y _beginlocation_z) (`KismetMathLibrary.BreakVector` (`self.beginLocation`)))
  (bind _returnvalue (`KismetMathLibrary.MakeVector` _beginlocation_x _beginlocation_y _beginlocation_z))
  (if (`|EnumInequality` (`self.animState`) "NewEnumerator2")
    (`GameplayStatics.PlaySound2D` "/Game/SoundEffects/mixkit-metallic-sword-strike-2160.mixkit-metallic-sword-strike-2160" 1.0 1.0 0.0 null null)
    (if (`self.IsComboActive`)
      (bind _result (`/Engine/EditorBlueprintResources/StandardMacros.IncrementInt` (`self.ComboCounter`))
        (:`  `
          (`KismetSystemLibrary.PrintString` (`KismetStringLibrary.Conv_IntToString` _result))
          (bind _returnvalue_2 (`|CreateWidget` "/Game/SpecialEffects/ComboWidget.ComboWidget_C" null _result))
          (bind _output_get (set `self.ComboWidget` _returnvalue_2))
          (`UserWidget.AddToViewport` _output_get 0)
          (`/Game/SpecialEffects/ComboWidget.FadeOutAnimEvent` _output_get)
          (`self.CE_PlayerGetScore`)
          (`GameplayStatics.SpawnEmitterAtLocation` "/Game/StarterContent/Particles/P_Explosion.P_Explosion" _returnvalue (struct) (8.0 8.0 8.0))
          (`GameplayStatics.PlayWorldCameraShake` "/Game/SpecialEffects/HitCameraShake.HitCameraShake_C" _returnvalue 0.0 100000.0)
          (`self.CE_Down`)))
      (else
        (set `self.IsComboActive` true)
        (bind _result_2 (`/Engine/EditorBlueprintResources/StandardMacros.IncrementInt` (`self.ComboCounter`))
          (:`  `
            (`KismetSystemLibrary.PrintString` (`KismetStringLibrary.Conv_IntToString` _result_2))))))
    (else
      (`GameplayStatics.PlaySound2D` "/Game/SoundEffects/mixkit-impact-of-a-blow-2150.mixkit-impact-of-a-blow-2150" 1.0 1.0 0.0 null null)
      (set `self.IsComboActive` false)
      (set `self.ComboCounter` 0))))

(event `CE_PlayerGetScore`
  (`/Game/Characters/BP_MultiplayerCharacter.CE_GetScore` (`self.bpMultiplayer`) (`self.playerScore`)))

(fn `RemoveWidget`
  (params (Widget :type "Widget Object Reference"))
  (`Widget.RemoveFromParent` Widget))

(fn `UserConstructionScript`)